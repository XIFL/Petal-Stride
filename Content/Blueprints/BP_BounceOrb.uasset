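; BP_BounceOrb is a flipbook-animated orb that detonates on any damage and respawns after a short delay.
; AnyDamage plays the detonate flipbook, then hides the actor and disables collision before calling Respawn.
; Respawn reuses the same actor, showing it with a respawn animation and restoring collision and idle once that finishes.
; An alternative DestroyandRespawn event, not called here, spawns a replacement at the transform saved on BeginPlay.
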(event `self.ReceiveBeginPlay`
  (set `self.RespawnLocation` (`self.GetTransform` self)))

(event `self.ReceiveTick`
  (params (DeltaSeconds :type "Float (single-precision)")))

(event `self.ReceiveAnyDamage`
  (params (Damage :type "Float (single-precision)") (DamageType :type "DamageType Object Reference") (InstigatedBy :type "Controller Object Reference") (DamageCauser :type "Actor Object Reference"))
  (set `self.Detonated` true)
  (`PaperFlipbookComponent.SetFlipbook` (`self.Sprite`) "/Game/Assets/Flipbooks/FB_BounceOrbDetonate.FB_BounceOrbDetonate")
  (`KismetSystemLibrary.Delay` 0.5)
  (`self.SetActorHiddenInGame` true)
  (`self.SetActorEnableCollision` false)
  (`KismetSystemLibrary.Delay` 2.5)
  (`self.Respawn`))

(event `Respawn`
  (if (`self.Detonated`)
    (set `self.Detonated` false)
    (`self.SetActorHiddenInGame` false)
    (`PaperFlipbookComponent.SetFlipbook` (`self.Sprite`) "/Game/Assets/Flipbooks/FB_BounceOrbRespawn.FB_BounceOrbRespawn")
    (`KismetSystemLibrary.Delay` 0.5)
    (`self.SetActorEnableCollision` true)
    (`PaperFlipbookComponent.SetFlipbook` (`self.Sprite`) "/Game/Assets/Flipbooks/FB_BounceOrbIdle.FB_BounceOrbIdle")))

(event `Destroy and Respawn`
  (if (`self.Detonated`)
    (`self.K2_DestroyActor`)
    (set `self.Detonated` false)
    (bind _returnvalue (`|SpawnActorFromClass` "BP_BounceOrb_C" (`self.RespawnLocation`) "Undefined" "MultiplyWithRoot" null null))
    (`PaperFlipbookComponent.SetFlipbook` (`PaperCharacter.Sprite` _returnvalue) "/Game/Assets/Flipbooks/FB_BounceOrbIdle.FB_BounceOrbIdle")))

(fn `UserConstructionScript`)